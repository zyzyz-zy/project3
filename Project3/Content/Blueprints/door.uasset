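; Door Blueprint that opens when enough pressure switches are active.
; SwitchActivated and SwitchDActivation events raise and lower an active-switch counter and compare it to the required count.
; Meeting the threshold plays the Dooropen timeline, which drives the Door component's relative Z location; falling below it reverses the timeline to close the door.
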(event `SwitchActivated`
  (`/Engine/EditorBlueprintResources/StandardMacros.IncrementInt` (`self.PressureSwitchActive`)
    (:`  `
      (if (>= (`self.PressureSwitchActive`) (`self.PressureSwitchNeeded`))
        (bind (_direction _door_position) (`Timeline|dooropen` :!label _label)
          (:`Update`
            (`SceneComponent.K2_SetRelativeLocation` (`self.door`) (`KismetMathLibrary.MakeVector` 0.0 0.0 _door_position) false false)))
        (else
          (goto _label :!via `Reverse`))))))

(event `SwitchDActivation`
  (`/Engine/EditorBlueprintResources/StandardMacros.DecrementInt` (`self.PressureSwitchActive`)
    (:`  `
      (if (>= (`self.PressureSwitchActive`) (`self.PressureSwitchNeeded`))
        (goto _label)
        (else
          (goto _label :!via `Reverse`))))))

(fn `UserConstructionScript`)