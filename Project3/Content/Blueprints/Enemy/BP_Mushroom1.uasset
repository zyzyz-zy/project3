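; Mushroom melee enemy that chases the player, attacks up close and may drop a health pickup when killed.
; A detection overlap starts a self-repeating AI move toward the player, while a timed loop plays the attack montage and applies delayed damage if the attack-range overlap is active.
; Damage spawns Niagara effects; at zero health it enables mesh physics, destroys itself and attempts loot at a nearby reachable point.
; Tick turns the health bar toward the player and updates it.
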(event `self.ReceiveBeginPlay`
  (`KismetSystemLibrary.RetriggerableDelay` 1.0 :!label _label)
  (`self.attacked player`)
  (goto _label))

(event `Chase player`
  (if (not (`self.isDead?`))
    (`|AIMoveTo` self (0.0 0.0 0.0) (`GameplayStatics.GetPlayerCharacter` 0) 120.0
      (:`OnSuccess`
        (`self.Chase player`)))))

(event `self.detection reviews.OnComponentBeginOverlap`
  (params (OverlappedComponent :type "PrimitiveComponent Object Reference") (OtherActor :type "Actor Object Reference") (OtherComp :type "PrimitiveComponent Object Reference") (OtherBodyIndex :type Integer) (bFromSweep :type Boolean) (SweepResult :type "HitResult Structure (by ref)"))
  (cast `/Game/ThirdPerson/Blueprints/BP_ThirdPersonCharacter` OtherActor)
  (`self.Chase player`))

(event `self.ReceiveAnyDamage`
  (params (Damage :type "Float (single-precision)") (DamageType :type "DamageType Object Reference") (InstigatedBy :type "Controller Object Reference") (DamageCauser :type "Actor Object Reference"))
  (set `self.health` (- (`self.health`) Damage))
  (`NiagaraFunctionLibrary.SpawnSystemAtLocation` "/Game/Niagara_systems/NS_damage.NS_damage" (`self.K2_GetActorLocation`) (struct) (1.0 1.0 1.0) true true "AutoRelease")
  (if (<= (`self.health`) 0.0)
    (`PrimitiveComponent.SetSimulatePhysics` (`self.Mesh`) true)
    (`MovementComponent.StopMovementImmediately` (`self.CharacterMovement`))
    (set `self.isDead?` true)
    (for _ (range 1)
      (`self.K2_DestroyActor`))
    (`self.drop loot`)))

(event `self.attack red view.OnComponentBeginOverlap`
  (params (OverlappedComponent :type "PrimitiveComponent Object Reference") (OtherActor :type "Actor Object Reference") (OtherComp :type "PrimitiveComponent Object Reference") (OtherBodyIndex :type Integer) (bFromSweep :type Boolean) (SweepResult :type "HitResult Structure (by ref)"))
  ;[1 1 1] attack player
  (cast `/Game/ThirdPerson/Blueprints/BP_ThirdPersonCharacter` OtherActor)
  (set `self.isinradius` true))

(event `self.attack red view.OnComponentEndOverlap`
  (params (OverlappedComponent :type "PrimitiveComponent Object Reference") (OtherActor :type "Actor Object Reference") (OtherComp :type "PrimitiveComponent Object Reference") (OtherBodyIndex :type Integer))
  ;[1 1 1] attack player
  (cast `/Game/ThirdPerson/Blueprints/BP_ThirdPersonCharacter` OtherActor)
  (set `self.isinradius` false))

(event `attacked player`
  ;[1 1 1] attack player
  (if (`self.isinradius`)
    (if (not (`self.isDead?`))
      (`self.PlayAnimMontage` "/Game/MonsterForSurvivalGame/Animation/PBR/Mushroom/AngryVersion/Mushroom_Attack02Angry_ANIM_Montage.Mushroom_Attack02Angry_ANIM_Montage")
      (`KismetSystemLibrary.Delay` 0.82)
      (bind _asbp_third_person_character (cast `/Game/ThirdPerson/Blueprints/BP_ThirdPersonCharacter` (`GameplayStatics.GetPlayerCharacter` 0)))
      (`GameplayStatics.ApplyDamage` _asbp_third_person_character 10.0)
      (`GameplayStatics.PlaySound2D` "/Engine/VREditor/Sounds/UI/Floating_UI_Close.Floating_UI_Close" 1.0 1.0 0.0 null null))))

(event `self.ReceiveTick`
  (params (DeltaSeconds :type "Float (single-precision)"))
  (`SceneComponent.K2_SetWorldRotation` (`self.Health Widget`) (`KismetMathLibrary.FindLookAtRotation` (`SceneComponent.K2_GetComponentLocation` (`self.Health Widget`)) (`self.K2_GetActorLocation` (`GameplayStatics.GetPlayerCharacter` 0))) false false)
  (bind _aswb_enemy_healthbar (cast `/Game/UI/WB_EnemyHealthbar` (`WidgetComponent.GetWidget` (`self.Health Widget`))))
  (`ProgressBar.SetPercent` (`/Game/UI/WB_EnemyHealthbar.health` _aswb_enemy_healthbar) (/ (`self.health`) 50.0)))

(event `drop loot`
  (bind _returnvalue (`self.K2_GetActorLocation`))
  (bind _outhit (`KismetSystemLibrary.LineTraceSingle` _returnvalue (- _returnvalue (0.0 0.0 200.0)) "TraceTypeQuery1" false (`|MakeArray` (`GameplayStatics.GetPlayerCharacter` 0) :!type "Actor Object Reference")))
  (`|SpawnActorFromClass` (select `int` (`KismetMathLibrary.RandomInteger` 3) :`0` "/Game/Blueprints/HealthCollector.HealthCollector_C" :`1` null :`2` null :`3` null :!type "Actor Class Reference") (`KismetMathLibrary.MakeTransform` (`NavigationSystemV1.K2_GetRandomReachablePointInRadius` (`.Location` (`GameplayStatics.BreakHitResult` _outhit)) 200.0 null null) (`KismetMathLibrary.MakeRotator` 0.0 0.0 (`KismetMathLibrary.RandomFloatInRange` 0.0 360.0))) "Undefined" "MultiplyWithRoot" null null))

(fn `UserConstructionScript`)